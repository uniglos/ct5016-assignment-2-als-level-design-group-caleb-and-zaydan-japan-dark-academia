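; Actor that removes itself from the level once the player is in range and holds the first key, likely acting as a key-gated barrier.
; Overlap begin and end events cast to BP_Player, caching the player reference and toggling an InRange flag.
; Tick polls the player's HasKey1 flag alongside InRange and destroys the actor when both are true.
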(event `self.ReceiveActorEndOverlap`
  (params (OtherActor :type "Actor Object Reference"))
  (cast `/Game/Blueprints/BP_Player` OtherActor)
  (set `self.InRange` false))

(event `self.ReceiveActorBeginOverlap`
  (params (OtherActor :type "Actor Object Reference"))
  (bind _asbp_player (cast `/Game/Blueprints/BP_Player` OtherActor))
  (set `self.InRange` true))

(event `self.ReceiveTick`
  (params (DeltaSeconds :type "Float (single-precision)"))
  (if (and (`/Game/Blueprints/BP_Player.HasKey1` (stale `self.ReceiveActorBeginOverlap` _asbp_player)) (`self.InRange`))
    (`self.K2_DestroyActor`)))

(fn `UserConstructionScript`)